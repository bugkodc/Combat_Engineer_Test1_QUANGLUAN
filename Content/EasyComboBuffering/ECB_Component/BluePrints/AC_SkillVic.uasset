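; AC_SkillVic is a component for the victim side of a skill, playing the victim's reaction montage and applying its fatal end.
; SetInit caches the mesh plus the Attribute, Skill and Combo references.
; PlayVicSkill plays the montage immediately, or for launches waits half the given duration, then plays it and triggers a launch hit through Combo.
; EndVIc applies a huge negative Health change through Attribute, effectively killing the victim.
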(event `self.ReceiveBeginPlay`)

(event `PlayVicSkill`
  (params (MontageToPlay :type "AnimMontage Object Reference") (LaunchVelocity :type "Vector Structure") (Launch :type Boolean) (Duration :type "Float (single-precision)"))
  (bind _returnvalue (`SkeletalMeshComponent.GetAnimInstance` (`self.Mesh`)))
  (if Launch
    (`KismetSystemLibrary.Delay` (/ Duration 2.0))
    (`AnimInstance.Montage_Play` _returnvalue MontageToPlay 1.0 "MontageLength" 0.0 true)
    (`/Game/EasyComboBuffering/ECB_Component/BluePrints/AC_EasyComboBuffering.LauchHit` (`self.Combo`) LaunchVelocity)
    (else
      (`AnimInstance.Montage_Play` _returnvalue MontageToPlay 1.0 "MontageLength" 0.0 true))))

(fn `EndVIc`
  (`/Game/CT_Components/AttributeSystem/Components/CT_Cmpt_Attribute.IncVariable` (`self.Attribute`) (struct :`TagName` "CT.Attribute.Dynamic.Health") -999.0))

(fn `SetInit`
  (params (Mesh :type "SkeletalMeshComponent Object Reference") (Attribute :type "/Game/CT_Components/AttributeSystem/Components/CT_Cmpt_Attribute Object Reference") (Skill :type "SceneComponent Object Reference") (Combo :type "/Game/EasyComboBuffering/ECB_Component/BluePrints/AC_EasyComboBuffering Object Reference"))
  (set `self.Mesh` Mesh)
  (set `self.Attribute` Attribute)
  (set `self.Skill` Skill)
  (set `self.Combo` Combo))