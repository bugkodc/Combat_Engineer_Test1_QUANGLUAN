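; Global combat function library that resolves physical and magic damage, critical hits, evasion and life steal, and shows floating text over actors.
; Each calculation reads tagged values from the actors' C_Attribute components, rolling damage and armor within min/max ranges.
; Pierce reduces armor, which scales damage by a diminishing 100/(100+armor) curve.
; FloatingText reuses a "Floating"-tagged widget component or creates a screen-space WBP_FloatingText on demand.
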(fn `CalculateCritical`
  (params (Type :type Name) (AttackActor :type "Actor Object Reference") (DamagedActor :type "Actor Object Reference"))
  (returns (ReturnValue :type "Float (double-precision)"))
  (locals (Local_AttackCmpt :type "/Game/CombatTest/Blueprints/Components/Attribute/C_Attribute Object Reference") (Local_DamagedCmpt :type "/Game/CombatTest/Blueprints/Components/Attribute/C_Attribute Object Reference") (Local_IsCritical :type Boolean))
  (set `local.Local_AttackCmpt` (`Actor.GetComponentByClass` AttackActor "/Game/CombatTest/Blueprints/Components/Attribute/C_Attribute.C_Attribute_C"))
  (set `local.Local_DamagedCmpt` (`Actor.GetComponentByClass` (`local.DamagedActor`) "/Game/CombatTest/Blueprints/Components/Attribute/C_Attribute.C_Attribute_C"))
  (set `local.Local_IsCritical` (>= (- (`/Game/CombatTest/Blueprints/Components/Attribute/C_Attribute.GetAttribute` (`local.Local_AttackCmpt`) (struct :`TagName` "CT.Attribute.Normal.CriticalChance")) (`/Game/CombatTest/Blueprints/Components/Attribute/C_Attribute.GetAttribute` (`local.Local_DamagedCmpt`) (struct :`TagName` "CT.Attribute.Normal.Tenacity"))) (`KismetMathLibrary.RandomFloatInRange` 0.0 1.0)))
  (return (`KismetMathLibrary.FMax` (`KismetMathLibrary.SelectFloat` (+ (`/Game/CombatTest/Blueprints/Components/Attribute/C_Attribute.GetAttribute` (`local.Local_AttackCmpt`) (struct :`TagName` "CT.Attribute.Normal.Critical")) 1.0) 1.0 (`local.Local_IsCritical`)) 1.0)))

(fn `CalculateDamage`
  (params (Type :type Name) (AttackActor :type "Actor Object Reference") (DamagedActor :type "Actor Object Reference"))
  (returns (ReturnValue :type "Float (double-precision)"))
  (locals (Local_Damage :type "Float (double-precision)" :default 0.0) (Local_AttackCmpt :type "/Game/CombatTest/Blueprints/Components/Attribute/C_Attribute Object Reference") (Local_DamagedCmpt :type "/Game/CombatTest/Blueprints/Components/Attribute/C_Attribute Object Reference") (Local_Armor :type "Float (double-precision)" :default 0.0) (Local_Pierce :type "Float (double-precision)" :default 0.0) (`Local_Pierce%` :type "Float (double-precision)" :default 0.0))
  (set `local.Local_AttackCmpt` (`Actor.GetComponentByClass` AttackActor "/Game/CombatTest/Blueprints/Components/Attribute/C_Attribute.C_Attribute_C"))
  (`|ExecutionSequence`
    (:`then_0`
      (switch `name` (`local.Type`)
        (:`Physical`
          (set `local.Local_Damage` (`KismetMathLibrary.RandomFloatInRange` (`/Game/CombatTest/Blueprints/Components/Attribute/C_Attribute.GetAttribute` (`local.Local_AttackCmpt`) (struct :`TagName` "CT.Attribute.Combat.Min_PhysicalDamage")) (`/Game/CombatTest/Blueprints/Components/Attribute/C_Attribute.GetAttribute` (`local.Local_AttackCmpt`) (struct :`TagName` "CT.Attribute.Combat.Max_PhysicalDamage"))))
          (set `local.Local_Pierce` (`/Game/CombatTest/Blueprints/Components/Attribute/C_Attribute.GetAttribute` (`local.Local_AttackCmpt`) (struct :`TagName` "CT.Attribute.Combat.ArmorPierce")))
          (set `local.Local_Pierce%` (`/Game/CombatTest/Blueprints/Components/Attribute/C_Attribute.GetAttribute` (`local.Local_AttackCmpt`) (struct :`TagName` "CT.Attribute.Combat.ArmorPierce%"))))
        (:`Magic`
          (set `local.Local_Damage` (`KismetMathLibrary.RandomFloatInRange` (`/Game/CombatTest/Blueprints/Components/Attribute/C_Attribute.GetAttribute` (`local.Local_AttackCmpt`) (struct :`TagName` "CT.Attribute.Combat.Min_MagicDamage")) (`/Game/CombatTest/Blueprints/Components/Attribute/C_Attribute.GetAttribute` (`local.Local_AttackCmpt`) (struct :`TagName` "CT.Attribute.Combat.Max_MagicDamage"))))
          (set `local.Local_Pierce` (`/Game/CombatTest/Blueprints/Components/Attribute/C_Attribute.GetAttribute` (`local.Local_AttackCmpt`) (struct :`TagName` "CT.Attribute.Combat.MagicPierce")))
          (set `local.Local_Pierce%` (`/Game/CombatTest/Blueprints/Components/Attribute/C_Attribute.GetAttribute` (`local.Local_AttackCmpt`) (struct :`TagName` "CT.Attribute.Combat.MagicPierce%"))))))
    (:`then_1`
      (bind _returnvalue (`self.SimpleDamage` (`local.Type`) (`local.Local_Damage`) (`local.Local_Pierce`) (`local.Local_Pierce%`) (`local.DamagedActor`)))
      (return _returnvalue))))

(fn `CalculateEvasion`
  (params (Type :type Name) (AttackActor :type "Actor Object Reference") (DamagedActor :type "Actor Object Reference"))
  (returns (ReturnValue :type Boolean))
  (locals (Local_AttackCmpt :type "/Game/CombatTest/Blueprints/Components/Attribute/C_Attribute Object Reference") (Local_DamagedCmpt :type "/Game/CombatTest/Blueprints/Components/Attribute/C_Attribute Object Reference") (Local_IsCritical :type Boolean))
  (set `local.Local_AttackCmpt` (`Actor.GetComponentByClass` AttackActor "/Game/CombatTest/Blueprints/Components/Attribute/C_Attribute.C_Attribute_C"))
  (set `local.Local_DamagedCmpt` (`Actor.GetComponentByClass` (`local.DamagedActor`) "/Game/CombatTest/Blueprints/Components/Attribute/C_Attribute.C_Attribute_C"))
  (return (>= (- (`/Game/CombatTest/Blueprints/Components/Attribute/C_Attribute.GetAttribute` (`local.Local_DamagedCmpt`) (struct :`TagName` "CT.Attribute.Normal.Evasion")) (`/Game/CombatTest/Blueprints/Components/Attribute/C_Attribute.GetAttribute` (`local.Local_AttackCmpt`) (struct :`TagName` "CT.Attribute.Normal.Accuracy"))) (`KismetMathLibrary.RandomFloatInRange` 0.0 1.0))))

(fn `CalculateLifeSteal`
  (params (Type :type Name) (AttackActor :type "Actor Object Reference") (Damage :type "Float (double-precision)"))
  (returns (ReturnValue :type "Float (double-precision)"))
  (locals (Local_AttackCmpt :type "/Game/CombatTest/Blueprints/Components/Attribute/C_Attribute Object Reference"))
  (set `local.Local_AttackCmpt` (`Actor.GetComponentByClass` AttackActor "/Game/CombatTest/Blueprints/Components/Attribute/C_Attribute.C_Attribute_C"))
  (switch `name` (`local.Type`)
    (:`Physical`
      (return (* (`/Game/CombatTest/Blueprints/Components/Attribute/C_Attribute.GetAttribute` (`local.Local_AttackCmpt`) (struct :`TagName` "CT.Attribute.Normal.Lifesteal")) (`local.Damage`))))
    (:`Magic`
      (return (* (`/Game/CombatTest/Blueprints/Components/Attribute/C_Attribute.GetAttribute` (`local.Local_AttackCmpt`) (struct :`TagName` "CT.Attribute.Normal.SpellVamp")) (`local.Damage`))))))

(fn `FloatingText`
  (params (Actor :type "Actor Object Reference") (Text :type Text) (TextureIcon :type "Texture2D Object Reference") (Color :type "LinearColor Structure") (FontSize :type Integer :default 42))
  (locals (Local_Widget :type "/Game/CombatTest/Blueprints/UI/Attribute/Floating/WBP_FloatingText Object Reference") (Local_WidgetCmpt :type "WidgetComponent Object Reference"))
  (`|ExecutionSequence`
    (:`then_0`
      (bind _output_get (set `local.Local_WidgetCmpt` (`|GetArrayItem` (`Actor.GetComponentsByTag` (`local.Actor`) "/Script/UMG.WidgetComponent" "Floating"))))
      (`/Engine/EditorBlueprintResources/StandardMacros.IsValid` _output_get
        (:`Is Valid`
          (bind _aswbp_floating_text (cast `/Game/CombatTest/Blueprints/UI/Attribute/Floating/WBP_FloatingText` (`WidgetComponent.GetWidget` (`local.Local_WidgetCmpt`))))
          (`/Game/CombatTest/Blueprints/UI/Attribute/Floating/WBP_FloatingText.TextFloating` _aswbp_floating_text (`local.Text`) (`local.Color`) (`local.TextureIcon`) (`local.FontSize`))
          (return))))
    (:`then_1`
      (bind _returnvalue (`|CreateWidget` "/Game/CombatTest/Blueprints/UI/Attribute/Floating/WBP_FloatingText.WBP_FloatingText_C"))
      (set `local.Local_Widget` _returnvalue)
      (bind _returnvalue_2 (`|AddComponentByClass` (`local.Actor`) "/Script/UMG.WidgetComponent" false (`KismetMathLibrary.MakeTransform` (0.0 0.0 0.0))))
      (bind _output_get_2 (set `local.Local_WidgetCmpt` _returnvalue_2))
      (set `ActorComponent.ComponentTags` (`|MakeArray` "Floating" :!type "Name") _output_get_2)
      (`WidgetComponent.SetWidget` (`local.Local_WidgetCmpt`) (`local.Local_Widget`))
      (`/Engine/EditorBlueprintResources/StandardMacros.IsValid` (`local.Local_Widget`)
        (:`Is Valid`
          (`/Game/CombatTest/Blueprints/UI/Attribute/Floating/WBP_FloatingText.TextFloating` (`local.Local_Widget`) (`local.Text`) (`local.Color`) (`local.TextureIcon`) (`local.FontSize`))
          (`WidgetComponent.SetDrawAtDesiredSize` (`local.Local_WidgetCmpt`) true)
          (`WidgetComponent.SetWidgetSpace` (`local.Local_WidgetCmpt`) "Screen")
          (`PrimitiveComponent.SetMaterial` (`local.Local_WidgetCmpt`) 0 "/Engine/EngineMaterials/Widget3DPassThrough_Masked_OneSided.Widget3DPassThrough_Masked_OneSided"))))))

(fn `SimpleDamage`
  (params (Type :type Name) (Damage :type "Float (double-precision)") (Pierce :type "Float (double-precision)") (`Pierce%` :type "Float (double-precision)") (DamagedActor :type "Actor Object Reference"))
  (returns (ReturnValue :type "Float (double-precision)"))
  (locals (Local_Damage :type "Float (double-precision)" :default 0.0) (Local_AttackCmpt :type "/Game/CombatTest/Blueprints/Components/Attribute/C_Attribute Object Reference") (Local_DamagedCmpt :type "/Game/CombatTest/Blueprints/Components/Attribute/C_Attribute Object Reference") (Local_Armor :type "Float (double-precision)" :default 0.0) (Local_Pierce :type "Float (double-precision)" :default 0.0) (`Local_Pierce%` :type "Float (double-precision)" :default 0.0))
  (set `local.Local_DamagedCmpt` (`Actor.GetComponentByClass` DamagedActor "/Game/CombatTest/Blueprints/Components/Attribute/C_Attribute.C_Attribute_C"))
  (`|ExecutionSequence`
    (:`then_0`
      (switch `name` (`local.Type`)
        (:`Physical`
          (set `local.Local_Armor` (`KismetMathLibrary.RandomFloatInRange` (`/Game/CombatTest/Blueprints/Components/Attribute/C_Attribute.GetAttribute` (`local.Local_DamagedCmpt`) (struct :`TagName` "CT.Attribute.Combat.Min_PhysicalArmor")) (`/Game/CombatTest/Blueprints/Components/Attribute/C_Attribute.GetAttribute` (`local.Local_DamagedCmpt`) (struct :`TagName` "CT.Attribute.Combat.Max_PhysicalArmor")))))
        (:`Magic`
          (set `local.Local_Armor` (`KismetMathLibrary.RandomFloatInRange` (`/Game/CombatTest/Blueprints/Components/Attribute/C_Attribute.GetAttribute` (`local.Local_DamagedCmpt`) (struct :`TagName` "CT.Attribute.Combat.Min_MagicArmor")) (`/Game/CombatTest/Blueprints/Components/Attribute/C_Attribute.GetAttribute` (`local.Local_DamagedCmpt`) (struct :`TagName` "CT.Attribute.Combat.Max_MagicArmor")))))))
    (:`then_2`
      (return (`KismetMathLibrary.Conv_IntToDouble` (`KismetMathLibrary.Round` (* (/ 100.0 (+ (* (`KismetMathLibrary.FMax` (- (`local.Local_Armor`) (`local.Pierce`))) (- 1.0 (`local.Pierce%`))) 100.0)) (`local.Damage`))))))))