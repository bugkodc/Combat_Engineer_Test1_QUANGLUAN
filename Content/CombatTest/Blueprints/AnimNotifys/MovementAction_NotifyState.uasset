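; Anim notify state that drives the owning actor's movement action over an animation window.
; On begin it sends its configured MovementAction to the owner through a Blueprint interface message.
; On end it reads the owner's current states and resets the action to a fixed enum entry only if it still matches, so a later change is not overwritten.
; The notify name displays the selected action.
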(fn `GetNotifyName`
  (returns (ReturnValue :type String))
  (return (`KismetStringLibrary.Concat_StrStr` "Movement Action: " (`|GetEnumeratorNameAsString` (`self.MovementAction`)))))

(fn `Received_NotifyBegin`
  (params (MeshComp :type "SkeletalMeshComponent Object Reference") (Animation :type "AnimSequenceBase Object Reference") (TotalDuration :type "Float (single-precision)") (EventReference :type "AnimNotifyEventReference Structure (by ref)"))
  (returns (ReturnValue :type Boolean))
  (message `/Game/CombatTest/Blueprints/Interfaces/Character_BPI.BPI_Set_MovementAction` (`ActorComponent.GetOwner` MeshComp) (`self.MovementAction`))
  (return false))

(fn `Received_NotifyEnd`
  (params (MeshComp :type "SkeletalMeshComponent Object Reference") (Animation :type "AnimSequenceBase Object Reference") (EventReference :type "AnimNotifyEventReference Structure (by ref)"))
  (returns (ReturnValue :type Boolean))
  (bind (_pawnmovementmode _movementstate _prevmovementstate _movementaction) (message `/Game/CombatTest/Blueprints/Interfaces/Character_BPI.BPI_Get_CurrentStates` (`ActorComponent.GetOwner` MeshComp)))
  (if (`|EnumEquality` _movementaction (`self.MovementAction`))
    (message `/Game/CombatTest/Blueprints/Interfaces/Character_BPI.BPI_Set_MovementAction` (`ActorComponent.GetOwner` (`local.MeshComp`)) "NewEnumerator4")
    (return false)
    (else
      (return false))))