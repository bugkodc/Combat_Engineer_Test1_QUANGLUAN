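; Anim notify state, displayed as "Early Blend Out", that stops its montage early while the notify window is active if the character's state warrants it.
; Each tick runs optional checks for a matching movement state, a matching stance or any movement input.
; The owning actor supplies these values through Blueprint interface calls, and a passing check stops the specified montage with a configurable blend-out time.
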(fn `GetNotifyName`
  (returns (ReturnValue :type String))
  (return "Early Blend Out"))

(fn `Received_NotifyTick`
  (params (MeshComp :type "SkeletalMeshComponent Object Reference") (Animation :type "AnimSequenceBase Object Reference") (FrameDeltaTime :type "Float (single-precision)") (EventReference :type "AnimNotifyEventReference Structure (by ref)"))
  (returns (ReturnValue :type Boolean))
  (locals (AnimInstance :type "AnimInstance Object Reference") (OwningActor :type "Actor Object Reference"))
  (set `local.AnimInstance` (`SkeletalMeshComponent.GetAnimInstance` MeshComp))
  (set `local.OwningActor` (`ActorComponent.GetOwner` MeshComp))
  (`|ExecutionSequence`
    (:`then_0`
      (if (`self.CheckMovementState`)
        (bind (_pawnmovementmode _movementstate) (message `/Game/CombatTest/Blueprints/Interfaces/Character_BPI.BPI_Get_CurrentStates` (`local.OwningActor`)))
        (if (== _movementstate (`self.MovementStateEquals`))
          (`AnimInstance.Montage_Stop` (`local.AnimInstance`) (`self.BlendOutTime`) (`self.ThisMontage`))
          (return true))))
    (:`then_1`
      (if (`self.CheckStance`)
        (bind (_pawnmovementmode_2 _movementstate_2 _prevmovementstate _movementaction _rotationmode _actualgait _actualstance) (message `/Game/CombatTest/Blueprints/Interfaces/Character_BPI.BPI_Get_CurrentStates` (`local.OwningActor`)))
        (if (`|EnumEquality` _actualstance (`self.StanceEquals`))
          (`AnimInstance.Montage_Stop` (`local.AnimInstance`) (`self.BlendOutTime`) (`self.ThisMontage`))
          (return true))))
    (:`then_2`
      (if (`self.CheckMovementInput`)
        (bind (_velocity _acceleration _movementinput _ismoving _hasmovementinput) (message `/Game/CombatTest/Blueprints/Interfaces/Character_BPI.BPI_Get_EssentialValues` (`local.OwningActor`)))
        (if _hasmovementinput
          (`AnimInstance.Montage_Stop` (`local.AnimInstance`) (`self.BlendOutTime`) (`self.ThisMontage`))
          (return true))))))