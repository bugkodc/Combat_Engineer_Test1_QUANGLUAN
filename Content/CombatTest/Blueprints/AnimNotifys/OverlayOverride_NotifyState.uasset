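; Anim notify state that temporarily sets an overlay override state on the animation instance during a montage or sequence window.
; On begin it sends the configured OverlayOverrideState to the AnimInstance through the BPI_SetOverlayOverrideState interface message, and on end it resets that state to zero.
; Its notify name displays the configured state value in the animation timeline.
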(fn `GetNotifyName`
  (returns (ReturnValue :type String))
  (return (`KismetStringLibrary.Concat_StrStr` "OverlayOverrideState: " (`KismetStringLibrary.Conv_IntToString` (`self.OverlayOverrideState`)))))

(fn `Received_NotifyBegin`
  (params (MeshComp :type "SkeletalMeshComponent Object Reference") (Animation :type "AnimSequenceBase Object Reference") (TotalDuration :type "Float (single-precision)") (EventReference :type "AnimNotifyEventReference Structure (by ref)"))
  (returns (ReturnValue :type Boolean))
  (message `/Game/CombatTest/Blueprints/Interfaces/Animation_BPI.BPI_SetOverlayOverrideState` (`SkeletalMeshComponent.GetAnimInstance` MeshComp) (`self.OverlayOverrideState`))
  (return false))

(fn `Received_NotifyEnd`
  (params (MeshComp :type "SkeletalMeshComponent Object Reference") (Animation :type "AnimSequenceBase Object Reference") (EventReference :type "AnimNotifyEventReference Structure (by ref)"))
  (returns (ReturnValue :type Boolean))
  (message `/Game/CombatTest/Blueprints/Interfaces/Animation_BPI.BPI_SetOverlayOverrideState` (`SkeletalMeshComponent.GetAnimInstance` MeshComp) 0)
  (return false))