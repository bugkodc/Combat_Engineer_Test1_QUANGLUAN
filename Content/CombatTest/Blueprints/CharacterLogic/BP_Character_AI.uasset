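; AI combat character that extends a parent character with a customizable body color scheme and a low-health state.
; The construction script creates dynamic materials per body part, then applies one solid color or skin and clothing colors chosen by shirt, pants, shoe and glove options.
; BeginPlay initializes the ACSkillVic component and hides the widget.
; CheckDeath shows the widget and enables the query-only box while health is low but nonzero.
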(event `self.ReceiveBeginPlay`
  (`parent.ReceiveBeginPlay`)
  (`/Game/CombatTest/Blueprints/Components/Combat/BluePrints/AC_SkillVic.SetInit` (`self.AC_SkillVic`) (`self.Mesh`) (`self.CT_Cmpt_Attribute`) (`self.Skill`) (`self.C_Combo`))
  (`SceneComponent.SetVisibility` (`self.Widget`) false false))

(fn `CheckDeath`
  (bind _returnvalue (`/Game/CombatTest/Blueprints/Components/Attribute/C_Attribute.GetVariable` (`self.CT_Cmpt_Attribute`) (struct :`TagName` "CT.Attribute.Dynamic.Health")))
  (bind _returnvalue_2 (and (<= _returnvalue 40.0) (not (== _returnvalue 0.0))))
  (`parent.CheckDeath`)
  (`PrimitiveComponent.SetCollisionEnabled` (`self.Box`) (select `bool` _returnvalue_2 :`false` "NoCollision" :`true` "QueryOnly" :!type "ECollisionEnabled Enum"))
  (`SceneComponent.SetVisibility` (`self.Widget`) _returnvalue_2 false))

(fn `HitAction`
  (params (MultiplyValue :type "Float (double-precision)") (LaunchVelocity :type "Vector Structure") (Weapon :type Boolean))
  (`parent.HitAction` MultiplyValue LaunchVelocity Weapon))

(fn `Set/ResetColors`
  (if (`self.SolidColor`)
    (`MaterialInstanceDynamic.SetVectorParameterValue` (`self.Head`) "BaseColor" (`self.DefaultColor`))
    (`MaterialInstanceDynamic.SetVectorParameterValue` (`self.Torso`) "BaseColor" (`self.DefaultColor`))
    (`MaterialInstanceDynamic.SetVectorParameterValue` (`self.Pelvis`) "BaseColor" (`self.DefaultColor`))
    (`MaterialInstanceDynamic.SetVectorParameterValue` (`self.Shoulder_L`) "BaseColor" (`self.DefaultColor`))
    (`MaterialInstanceDynamic.SetVectorParameterValue` (`self.UpperArm_L`) "BaseColor" (`self.DefaultColor`))
    (`MaterialInstanceDynamic.SetVectorParameterValue` (`self.LowerArm_L`) "BaseColor" (`self.DefaultColor`))
    (`MaterialInstanceDynamic.SetVectorParameterValue` (`self.Hand_L`) "BaseColor" (`self.DefaultColor`))
    (`MaterialInstanceDynamic.SetVectorParameterValue` (`self.Shoulder_R`) "BaseColor" (`self.DefaultColor`))
    (`MaterialInstanceDynamic.SetVectorParameterValue` (`self.UpperArm_R`) "BaseColor" (`self.DefaultColor`))
    (`MaterialInstanceDynamic.SetVectorParameterValue` (`self.LowerArm_R`) "BaseColor" (`self.DefaultColor`))
    (`MaterialInstanceDynamic.SetVectorParameterValue` (`self.Hand_R`) "BaseColor" (`self.DefaultColor`))
    (`MaterialInstanceDynamic.SetVectorParameterValue` (`self.UpperLegs`) "BaseColor" (`self.DefaultColor`))
    (`MaterialInstanceDynamic.SetVectorParameterValue` (`self.LowerLegs`) "BaseColor" (`self.DefaultColor`))
    (`MaterialInstanceDynamic.SetVectorParameterValue` (`self.Feet`) "BaseColor" (`self.DefaultColor`))
    (else
      (`|ExecutionSequence`
        (:`then_0`
          (`MaterialInstanceDynamic.SetVectorParameterValue` (`self.Head`) "BaseColor" (`self.SkinColor`)))
        (:`then_1`
          (switch `int` (`self.ShirtType`)
            (:`0`
              (`MaterialInstanceDynamic.SetVectorParameterValue` (`self.Shoulder_L`) "BaseColor" (`self.SkinColor`))
              (`MaterialInstanceDynamic.SetVectorParameterValue` (`self.Shoulder_R`) "BaseColor" (`self.SkinColor`))
              (`MaterialInstanceDynamic.SetVectorParameterValue` (`self.UpperArm_L`) "BaseColor" (`self.SkinColor`))
              (`MaterialInstanceDynamic.SetVectorParameterValue` (`self.UpperArm_R`) "BaseColor" (`self.SkinColor`))
              (`MaterialInstanceDynamic.SetVectorParameterValue` (`self.LowerArm_L`) "BaseColor" (`self.SkinColor`))
              (`MaterialInstanceDynamic.SetVectorParameterValue` (`self.LowerArm_R`) "BaseColor" (`self.SkinColor`))
              (`MaterialInstanceDynamic.SetVectorParameterValue` (`self.Torso`) "BaseColor" (`self.SkinColor`)))
            (:`1`
              (`MaterialInstanceDynamic.SetVectorParameterValue` (`self.Shoulder_L`) "BaseColor" (`self.ShirtColor`))
              (`MaterialInstanceDynamic.SetVectorParameterValue` (`self.Shoulder_R`) "BaseColor" (`self.ShirtColor`))
              (`MaterialInstanceDynamic.SetVectorParameterValue` (`self.Torso`) "BaseColor" (`self.ShirtColor`))
              (`MaterialInstanceDynamic.SetVectorParameterValue` (`self.UpperArm_L`) "BaseColor" (`self.SkinColor`))
              (`MaterialInstanceDynamic.SetVectorParameterValue` (`self.UpperArm_R`) "BaseColor" (`self.SkinColor`))
              (`MaterialInstanceDynamic.SetVectorParameterValue` (`self.LowerArm_L`) "BaseColor" (`self.SkinColor`))
              (`MaterialInstanceDynamic.SetVectorParameterValue` (`self.LowerArm_R`) "BaseColor" (`self.SkinColor`)))
            (:`2`
              (`MaterialInstanceDynamic.SetVectorParameterValue` (`self.Shoulder_L`) "BaseColor" (`self.ShirtColor`))
              (`MaterialInstanceDynamic.SetVectorParameterValue` (`self.Shoulder_R`) "BaseColor" (`self.ShirtColor`))
              (`MaterialInstanceDynamic.SetVectorParameterValue` (`self.UpperArm_L`) "BaseColor" (`self.ShirtColor`))
              (`MaterialInstanceDynamic.SetVectorParameterValue` (`self.UpperArm_R`) "BaseColor" (`self.ShirtColor`))
              (`MaterialInstanceDynamic.SetVectorParameterValue` (`self.Torso`) "BaseColor" (`self.ShirtColor`))
              (`MaterialInstanceDynamic.SetVectorParameterValue` (`self.LowerArm_L`) "BaseColor" (`self.SkinColor`))
              (`MaterialInstanceDynamic.SetVectorParameterValue` (`self.LowerArm_R`) "BaseColor" (`self.SkinColor`)))
            (:`3`
              (`MaterialInstanceDynamic.SetVectorParameterValue` (`self.Shoulder_L`) "BaseColor" (`self.ShirtColor`))
              (`MaterialInstanceDynamic.SetVectorParameterValue` (`self.Shoulder_R`) "BaseColor" (`self.ShirtColor`))
              (`MaterialInstanceDynamic.SetVectorParameterValue` (`self.UpperArm_L`) "BaseColor" (`self.ShirtColor`))
              (`MaterialInstanceDynamic.SetVectorParameterValue` (`self.UpperArm_R`) "BaseColor" (`self.ShirtColor`))
              (`MaterialInstanceDynamic.SetVectorParameterValue` (`self.LowerArm_L`) "BaseColor" (`self.ShirtColor`))
              (`MaterialInstanceDynamic.SetVectorParameterValue` (`self.LowerArm_R`) "BaseColor" (`self.ShirtColor`))
              (`MaterialInstanceDynamic.SetVectorParameterValue` (`self.Torso`) "BaseColor" (`self.ShirtColor`)))))
        (:`then_2`
          (switch `int` (`self.PantsType`)
            (:`0`
              (`MaterialInstanceDynamic.SetVectorParameterValue` (`self.Pelvis`) "BaseColor" (`self.PantsColor`))
              (`MaterialInstanceDynamic.SetVectorParameterValue` (`self.UpperLegs`) "BaseColor" (`self.SkinColor`))
              (`MaterialInstanceDynamic.SetVectorParameterValue` (`self.LowerLegs`) "BaseColor" (`self.SkinColor`)))
            (:`1`
              (`MaterialInstanceDynamic.SetVectorParameterValue` (`self.Pelvis`) "BaseColor" (`self.PantsColor`))
              (`MaterialInstanceDynamic.SetVectorParameterValue` (`self.UpperLegs`) "BaseColor" (`self.PantsColor`))
              (`MaterialInstanceDynamic.SetVectorParameterValue` (`self.LowerLegs`) "BaseColor" (`self.SkinColor`)))
            (:`2`
              (`MaterialInstanceDynamic.SetVectorParameterValue` (`self.Pelvis`) "BaseColor" (`self.PantsColor`))
              (`MaterialInstanceDynamic.SetVectorParameterValue` (`self.UpperLegs`) "BaseColor" (`self.PantsColor`))
              (`MaterialInstanceDynamic.SetVectorParameterValue` (`self.LowerLegs`) "BaseColor" (`self.PantsColor`)))))
        (:`then_3`
          (if (`self.Shoes`)
            (`MaterialInstanceDynamic.SetVectorParameterValue` (`self.Feet`) "BaseColor" (`self.ShoesColor`))
            (else
              (`MaterialInstanceDynamic.SetVectorParameterValue` (`self.Feet`) "BaseColor" (`self.SkinColor`)))))
        (:`then_4`
          (if (`self.Gloves`)
            (`MaterialInstanceDynamic.SetVectorParameterValue` (`self.Hand_L`) "BaseColor" (`self.GlovesColor`))
            (`MaterialInstanceDynamic.SetVectorParameterValue` (`self.Hand_R`) "BaseColor" (`self.GlovesColor`))
            (else
              (`MaterialInstanceDynamic.SetVectorParameterValue` (`self.Hand_L`) "BaseColor" (`self.SkinColor`))
              (`MaterialInstanceDynamic.SetVectorParameterValue` (`self.Hand_R`) "BaseColor" (`self.SkinColor`)))))))))

(fn `SetDynamicMaterials`
  (`|ExecutionSequence`
    (:`then_0`
      (bind _returnvalue (`PrimitiveComponent.CreateDynamicMaterialInstance` (`self.Mesh`) 2 null "None"))
      (set `self.Head` _returnvalue)
      (bind _returnvalue_2 (`PrimitiveComponent.CreateDynamicMaterialInstance` (`self.Mesh`) 1 null "None"))
      (set `self.Torso` _returnvalue_2)
      (bind _returnvalue_3 (`PrimitiveComponent.CreateDynamicMaterialInstance` (`self.Mesh`) 0 null "None"))
      (set `self.Pelvis` _returnvalue_3))
    (:`then_1`
      (bind _returnvalue_4 (`PrimitiveComponent.CreateDynamicMaterialInstance` (`self.Mesh`) 6 null "None"))
      (set `self.UpperLegs` _returnvalue_4)
      (bind _returnvalue_5 (`PrimitiveComponent.CreateDynamicMaterialInstance` (`self.Mesh`) 7 null "None"))
      (set `self.LowerLegs` _returnvalue_5)
      (bind _returnvalue_6 (`PrimitiveComponent.CreateDynamicMaterialInstance` (`self.Mesh`) 8 null "None"))
      (set `self.Feet` _returnvalue_6))
    (:`then_2`
      (bind _returnvalue_7 (`PrimitiveComponent.CreateDynamicMaterialInstance` (`self.Mesh`) 4 null "None"))
      (set `self.Shoulder_L` _returnvalue_7)
      (bind _returnvalue_8 (`PrimitiveComponent.CreateDynamicMaterialInstance` (`self.Mesh`) 3 null "None"))
      (set `self.UpperArm_L` _returnvalue_8)
      (bind _returnvalue_9 (`PrimitiveComponent.CreateDynamicMaterialInstance` (`self.Mesh`) 5 null "None"))
      (set `self.LowerArm_L` _returnvalue_9)
      (bind _returnvalue_10 (`PrimitiveComponent.CreateDynamicMaterialInstance` (`self.Mesh`) 9 null "None"))
      (set `self.Hand_L` _returnvalue_10))
    (:`then_3`
      (bind _returnvalue_11 (`PrimitiveComponent.CreateDynamicMaterialInstance` (`self.Mesh`) 12 null "None"))
      (set `self.Shoulder_R` _returnvalue_11)
      (bind _returnvalue_12 (`PrimitiveComponent.CreateDynamicMaterialInstance` (`self.Mesh`) 11 null "None"))
      (set `self.UpperArm_R` _returnvalue_12)
      (bind _returnvalue_13 (`PrimitiveComponent.CreateDynamicMaterialInstance` (`self.Mesh`) 13 null "None"))
      (set `self.LowerArm_R` _returnvalue_13)
      (bind _returnvalue_14 (`PrimitiveComponent.CreateDynamicMaterialInstance` (`self.Mesh`) 14 null "None"))
      (set `self.Hand_R` _returnvalue_14))))

(fn `UserConstructionScript`
  (`parent.UserConstructionScript`)
  (`self.SetDynamicMaterials`)
  (`self.Set/ResetColors`))