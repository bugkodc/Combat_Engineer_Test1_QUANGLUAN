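; SaveGame Blueprint that holds a SavedData map for attribute data, with AddValue writing entries by key and GetValue looking them up by SaveID.
; Save writes the object to a slot if the given actor has a C_Attribute component, but its map-add node is unconnected.
; Delay_SaveGameToSlot defers the slot write through a short timer.
; Load is an empty stub.
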(event `Delay_SaveGameToSlot`
  (params (SlotName :type String) (UserIndex :type Integer))
  (`KismetSystemLibrary.K2_SetTimerDelegate` (delegate `CustomEvent`) 0.1))

(event `CustomEvent`
  (`GameplayStatics.SaveGameToSlot` self (stale `Delay_SaveGameToSlot` SlotName) (stale `Delay_SaveGameToSlot` UserIndex)))

(fn `AddValue`
  (params (Key :type "Name (by ref)") (Value :type "/Game/CombatTest/Data/Structs/S_Save_Attributes Structure (by ref)"))
  (`BlueprintMapLibrary.Map_Add` (`self.SavedData`) Key Value))

(fn `GetValue`
  (params (SaveID :type "Name (by ref)"))
  (returns (Value :type "/Game/CombatTest/Data/Structs/S_Save_Attributes Structure") (ReturnValue :type Boolean))
  (bind (_value _returnvalue) (`BlueprintMapLibrary.Map_Find` (`self.SavedData`) SaveID))
  (return _value _returnvalue))

(fn `Load`)

(fn `Save`
  (params (Actor :type "Actor Object Reference") (SaveID :type Name) (SlotName :type String) (UserIndex :type Integer))
  (`/Engine/EditorBlueprintResources/StandardMacros.IsValid` (`Actor.GetComponentByClass` Actor "/Game/CombatTest/Blueprints/Components/Attribute/C_Attribute.C_Attribute_C")
    (:`Is Valid`
      (`GameplayStatics.SaveGameToSlot` self (`local.SlotName`) (`local.UserIndex`)))))