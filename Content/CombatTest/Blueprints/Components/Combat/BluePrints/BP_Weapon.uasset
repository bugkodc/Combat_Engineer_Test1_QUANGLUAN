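; BP_Weapon is a data-driven weapon actor with a mesh and a Niagara effect that samples that mesh.
; The construction script loads its DT_WeaponState row; BeginPlay applies it and, for dual weapons, spawns BP_2ndWeapon on the owner's holster socket.
; ShowHidenWeapon sets visibility on both weapons.
; ChangeNiagara picks a random effect and writes the same-index color to a Material Parameter Collection.
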(event `self.ReceiveBeginPlay`
  (bind _niagara (`self.Niagara`))
  (bind ((`WeaponMesh_5_2D560EC24D796E524B28D1B0DD1C0D68` _weaponmesh) (`Niagara_Weapon_1_62_A5BEE6774414A2476E6B308904FCAF62` _niagara_weapon_1) (`IsDualWeapon_37_8B09CBA4451BDE883F5A6F80881C715C` _isdualweapon) (`2ndWeaponMesh_40_ACB81C2149288706D56E298D03E89E3B` _2ndweaponmesh)) (break `/Game/CombatTest/Blueprints/Components/Combat/Structures/F_WeaponStruct` (`.WeaponSetup_63_81966DAD4E20AB34F2E4139A7F332367` (break `/Game/CombatTest/Blueprints/Components/Combat/Structures/F_WeaponState` (`self.WeaponData`)))))
  (`StaticMeshComponent.SetStaticMesh` (`self.WeaponMesh`) _weaponmesh)
  (`NiagaraComponent.SetAsset` _niagara _niagara_weapon_1 true)
  (`NiagaraComponent.SetVariableStaticMesh` _niagara "01 - Mesh -> Weapon" _weaponmesh)
  (if _isdualweapon
    (bind _returnvalue (`|SpawnActorFromClass` "/Game/CombatTest/Blueprints/Components/Combat/BluePrints/BP_2ndWeapon.BP_2ndWeapon_C" (`KismetMathLibrary.MakeTransform` (0.0 0.0 0.0)) "Undefined" "OverrideRootScale" (`self.GetOwner`) _2ndweaponmesh null))
    (set `self.2ndWeapon` _returnvalue)
    (`self.K2_AttachToComponent` (`self.2ndWeapon`) (`self.GetComponentByClass` (`self.GetOwner`) "/Script/Engine.SkeletalMeshComponent") (`.2ndHolsterSocket_47_81966DAD4E20AB34F2E4139A7F332367` (break `/Game/CombatTest/Blueprints/Components/Combat/Structures/F_WeaponStruct` (`.WeaponSetup_63_81966DAD4E20AB34F2E4139A7F332367` (break `/Game/CombatTest/Blueprints/Components/Combat/Structures/F_WeaponState` (`self.WeaponData`))))) "SnapToTarget" "SnapToTarget" "KeepRelative" true)))

(fn `ChangeNiagara`
  (locals (RandomIndex :type Integer :default 0))
  (bind _niagara (`self.Niagara`))
  (bind _arrayniagara (`self.ArrayNiagara`))
  (set `local.RandomIndex` (`KismetMathLibrary.RandomIntegerInRange` 0 (- (`KismetArrayLibrary.Array_Length` _arrayniagara) 1)))
  (`NiagaraComponent.SetAsset` _niagara (`|GetArrayItem` _arrayniagara (`local.RandomIndex`)) true)
  (`NiagaraComponent.SetVariableStaticMesh` _niagara "01 - Mesh -> Weapon" (`StaticMeshComponent.StaticMesh` (`self.WeaponMesh`)))
  (`KismetMaterialLibrary.SetVectorParameterValue` "/Game/CombatTest/Materials/FX_Materials/MP_ChangColorWeapon.MP_ChangColorWeapon" "Color" (`|GetArrayItem` (`self.Parameter Value`) (`local.RandomIndex`))))

(fn `Show_HidenWeapon`
  (params (bNewHidden :type Boolean))
  (`self.SetActorHiddenInGame` bNewHidden)
  (bind _2ndweapon (`self.2ndWeapon`)
    (:`then`
      (`self.SetActorHiddenInGame` _2ndweapon bNewHidden))
    (:`else`)))

(fn `UserConstructionScript`
  (bind _returnvalue (`|GetDataTableRow` "/Game/CombatTest/Blueprints/Components/Combat/DataTables/DT_WeaponState.DT_WeaponState" (`.WeaponName_3_E4A4170B4A4E8207B028ABBF182047A4` (break `/Game/CombatTest/Blueprints/Components/Combat/Structures/F_StoredWeapons` (`self.StoredWeapon`))))
    (:`then`
      (set `self.WeaponData` _returnvalue))))